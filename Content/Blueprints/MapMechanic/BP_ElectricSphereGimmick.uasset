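; Electric sphere map gimmick that drives its NovaFX effect to match the current stage and radius.
; OnStageChanged passes the stage (offset by one), elapsed time and radius to the effect's User parameters, then activates it without a reset.
; It backdates the phase start by the stage's age, so the visual picks up mid-stage.
; Tick keeps updating the elapsed time, capped at two seconds.
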(event `self.OnStageChanged`
  (params (NewStage :type "EHALElectricSphereStage Enum" :default "Begin") (StageAgeSeconds :type "Float (single-precision)") (StageDurationSeconds :type "Float (single-precision)") (RadiusCm :type "Float (single-precision)"))
  (bind _novafx (`self.NovaFX`))
  (set `self.PhaseStartTime` (- (`KismetSystemLibrary.GetGameTimeInSeconds`) StageAgeSeconds))
  (`NiagaraComponent.SetVariableInt` _novafx "User.Phase" (+ (`KismetMathLibrary.Conv_ByteToInt` NewStage) 1))
  (`NiagaraComponent.SetVariableFloat` _novafx "User.PhaseElapsed" (`KismetMathLibrary.FMin` StageAgeSeconds 2.0))
  (`NiagaraComponent.SetVariableFloat` _novafx "User.Radius" RadiusCm)
  (`ActorComponent.Activate` _novafx false))

(event `self.ReceiveTick`
  (params (DeltaSeconds :type "Float (single-precision)"))
  (`NiagaraComponent.SetVariableFloat` (`self.NovaFX`) "User.PhaseElapsed" (`KismetMathLibrary.FMin` (- (`KismetSystemLibrary.GetGameTimeInSeconds`) (`self.PhaseStartTime`)) 2.0)))

(fn `UserConstructionScript`)