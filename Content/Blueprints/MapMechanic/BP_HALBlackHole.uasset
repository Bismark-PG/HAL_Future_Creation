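; BP_HALBlackHole is the visual layer for a black hole map mechanic, driving Niagara effects from field, pulse and stage events.
; Field updates cache the radius and swirl direction, then push them with preparation progress into the FieldFX component.
; Each attraction pulse spawns a pulse system with raised translucent sort priority, and stage 2 spawns an over effect, both fed the cached radius and swirl sign.
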(event `self.OnFieldUpdated`
  (params (RadiusCm :type "Float (single-precision)") (PreparationProgress :type "Float (single-precision)"))
  (bind _fieldfx (`self.FieldFX`))
  (bind _returnvalue (`KismetMathLibrary.SelectFloat` -1.0 1.0 (== (`.SwirlDirection` (break `HALBlackHoleConfig` (`self.Settings`))) 1)))
  (set `self.LastRadius` RadiusCm)
  (set `self.SwirlSign` _returnvalue)
  (`NiagaraComponent.SetVariableFloat` _fieldfx "User.Radius" RadiusCm)
  (`NiagaraComponent.SetVariableFloat` _fieldfx "User.Preparation" PreparationProgress)
  (`NiagaraComponent.SetVariableFloat` _fieldfx "User.SwirlSign" _returnvalue))

(event `self.OnAttractionPulse`
  (params (NewPulseIndex :type Integer))
  (bind _returnvalue (`NiagaraFunctionLibrary.SpawnSystemAtLocation` "/Game/Assets/FX/NS_BlackHole_Pulse.NS_BlackHole_Pulse" (`self.K2_GetActorLocation`)))
  (if (`KismetSystemLibrary.IsValid` _returnvalue)
    (`NiagaraComponent.SetVariableFloat` _returnvalue "User.Radius" (`self.LastRadius`))
    (`NiagaraComponent.SetVariableFloat` _returnvalue "User.SwirlSign" (`self.SwirlSign`))
    (`PrimitiveComponent.SetTranslucentSortPriority` _returnvalue 1)))

(event `self.OnStageChanged`
  (params (NewStage :type "EHALBlackHoleStage Enum" :default "Expanding"))
  (if (== NewStage 2)
    (bind _returnvalue (`NiagaraFunctionLibrary.SpawnSystemAtLocation` "/Game/Assets/FX/NS_BlackHole_Over.NS_BlackHole_Over" (`self.K2_GetActorLocation`)))
    (if (`KismetSystemLibrary.IsValid` _returnvalue)
      (`NiagaraComponent.SetVariableFloat` _returnvalue "User.Radius" (`self.LastRadius`))
      (`NiagaraComponent.SetVariableFloat` _returnvalue "User.SwirlSign" (`self.SwirlSign`)))))

(fn `UserConstructionScript`)